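; T3Door_BP is a key-locked sliding door that opens for the third-person character.
; Box overlap begin checks the character's HasKey flag, printing a warning if it is missing.
; End overlap reenters that check, reusing the last cast, so a shared FlipFlop alternates between playing the Timeline and reversing it after a delay.
; The Timeline lerps the Door's relative location sideways along X.
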(event `self.Box.OnComponentBeginOverlap`
  (params (OverlappedComponent :type "PrimitiveComponent Object Reference") (OtherActor :type "Actor Object Reference") (OtherComp :type "PrimitiveComponent Object Reference") (OtherBodyIndex :type Integer) (bFromSweep :type Boolean) (SweepResult :type "HitResult Structure (by ref)"))
  ;[1 0.8201 0.05535] Open The Door
  (bind _asbp_third_person_character (cast `/Game/ThirdPerson/Blueprints/BP_ThirdPersonCharacter` OtherActor))
  (if (`/Game/ThirdPerson/Blueprints/BP_ThirdPersonCharacter.HasKey?` _asbp_third_person_character) :!label _label
    (`/Engine/EditorBlueprintResources/StandardMacros.FlipFlop`
      (:`A`
        (bind (_direction _speed) (`Timeline|Timeline` :!label _label_2)
          (:`Update`
            (`SceneComponent.K2_SetRelativeLocation` (`self.Door`) (`KismetMathLibrary.VLerp` (0.0 0.0 0.0) (200.0 0.0 0.0) _speed) false false))))
      (:`B`
        (`KismetSystemLibrary.Delay` 3.0)
        (goto _label_2 :!via `Reverse`)))
    (else
      (`KismetSystemLibrary.PrintString` "No Key,Please get the key first"))))

(event `self.Box.OnComponentEndOverlap`
  (params (OverlappedComponent :type "PrimitiveComponent Object Reference") (OtherActor :type "Actor Object Reference") (OtherComp :type "PrimitiveComponent Object Reference") (OtherBodyIndex :type Integer))
  ;[1 0.8201 0.05535] Open The Door
  (goto _label))

(fn `UserConstructionScript`)